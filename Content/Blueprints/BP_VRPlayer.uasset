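; BP_VRPlayer is a VR player pawn that handles smooth, thumbstick-driven locomotion.
; The left motion controller thumbstick's X and Y axes feed AddMovementInput, scaled by MovementSpeed, for strafing and forward/backward movement.
; Direction follows the camera's right and forward vectors with Z zeroed, keeping movement horizontal; the vectors are not renormalized, so looking up or down shortens the forward input.
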(event `InputAxis|MotionControllerThumbLeft_X`
  (params (AxisValue :type "Float (single-precision)"))
  (bind (_returnvalue_x _returnvalue_y) (`KismetMathLibrary.BreakVector` (`SceneComponent.GetRightVector` (`self.Camera`))))
  ;[1 1 1] Movement
  ;;[1 1 1] Left and Right Movement
  (if (not (== AxisValue 0.0))
    (`self.AddMovementInput` (`KismetMathLibrary.MakeVector` _returnvalue_x _returnvalue_y) (* AxisValue (`self.Movement Speed`)))))

(event `InputAxis|MotionControllerThumbLeft_Y`
  (params (AxisValue :type "Float (single-precision)"))
  (bind (_returnvalue_x _returnvalue_y) (`KismetMathLibrary.BreakVector` (`SceneComponent.GetForwardVector` (`self.Camera`))))
  ;[1 1 1] Movement
  ;;[1 1 1] Forward and Backward Movement
  (if (not (== AxisValue 0.0))
    (`self.AddMovementInput` (`KismetMathLibrary.MakeVector` _returnvalue_x _returnvalue_y) (* AxisValue (`self.Movement Speed`)))))

(fn `UserConstructionScript`)